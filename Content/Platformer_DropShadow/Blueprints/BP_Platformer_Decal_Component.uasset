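; Platformer drop shadow component that projects a circle decal on the ground beneath a character to show where they are above it.
; The owning character passes itself in through an initialize event, and a begin play event spawns the decal at its mesh.
; The tick event traces down from the mesh on Visibility, moves the decal to the impact height, and scales it by clamped hit distance, collapsing it to zero when nearly grounded.
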(event `Initalize Platformer Component`
  (params (Character :type "Character Object Reference"))
  ; In your players construction script or your event begin play, call this fuction and pass a reference to your player into it.
  (set `self.Character` Character))

(event `Platformer Component Begin Play`
  ;[1 1 1] Spawn Decal when gameplay begins.
  ; Call this function at the players event begin play.
  (bind _returnvalue (`GameplayStatics.SpawnDecalAtLocation` "/Game/Platformer_DropShadow/Materials/M_Decal_Circle.M_Decal_Circle" (16.0 64.0 64.0) (`SceneComponent.K2_GetComponentLocation` (`Character.Mesh` (`self.Character`)))))
  (set `self.Platformer Decal` _returnvalue))

(event `Platformer Component Tick`
  (bind _returnvalue (`KismetMathLibrary.MapRangeClamped` (`self.Line Trace Hit Distance`) 16.0 256.0 0.0 0.5))
  (bind (_returnvalue_x _returnvalue_y) (`KismetMathLibrary.BreakVector` (`Actor.K2_GetActorLocation` (`self.Character`))))
  (bind _returnvalue_2 (`SceneComponent.K2_GetComponentLocation` (`Character.Mesh` (`self.Character`))))
  ;[1 1 1] Platformer Drop Shadow:
  ; Every Frame perform a line trace from the player toward the ground.
  ; Scale the decal based on the players distance from the ground while also limiting the max size.
  ;
  ; Ground State = 0.150006
  (bind _outhit (`KismetSystemLibrary.LineTraceSingle` _returnvalue_2 (`KismetMathLibrary.MakeVector` (.x _returnvalue_2) (.y _returnvalue_2) -1024.0) "TraceTypeQuery1"))
  (bind _output_get (set `self.Out Hit` _outhit))
  (set `self.Line Trace Hit Distance` (`.Distance` (`GameplayStatics.BreakHitResult` _output_get)))
  (`SceneComponent.K2_SetWorldTransform` (`self.Platformer Decal`) (`KismetMathLibrary.MakeTransform` (`KismetMathLibrary.MakeVector` _returnvalue_x _returnvalue_y (.z (`.ImpactPoint` (`GameplayStatics.BreakHitResult` _output_get)))) (struct :`Pitch` -90.0) (`KismetMathLibrary.SelectVector` (0.0 0.0 0.0) (`KismetMathLibrary.MakeVector` 1.0 _returnvalue _returnvalue) (<= (`self.Line Trace Hit Distance`) 2.54))) false false))