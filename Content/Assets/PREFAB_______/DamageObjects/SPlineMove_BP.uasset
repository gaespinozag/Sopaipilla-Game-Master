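; Spline mover Blueprint that carries a referenced Actor along its spline in a continuous loop.
; The construction script places the Actor at the first spline point.
; On BeginPlay, a Timeline with play rate set from TimelineLenght lerps distance to the last point, updating world location without sweep and restarting from the start when finished.
; Tangent-based rotation logic exists but is not connected.
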(event `self.ReceiveBeginPlay`
  (`TimelineComponent.SetPlayRate` (`self.Timeline`) (/ 1.0 (`self.Timeline Lenght`)))
  (`self.Play Timeline`))

(event `Play Timeline`
  (bind _spline (`self.Spline`))
  (bind (_direction _newtrack_0) (`Timeline|Timeline` :!via `PlayFromStart`)
    (:`Update`
      (`self.K2_SetActorLocation` (`self.Actor`) (`SplineComponent.GetLocationAtDistanceAlongSpline` (`self.Spline`) (`KismetMathLibrary.Lerp` 0.0 (`SplineComponent.GetDistanceAlongSplineAtSplinePoint` _spline (- (`SplineComponent.GetNumberOfSplinePoints` _spline) 1)) _newtrack_0) "World") false false))
    (:`Finished`
      (`self.Play Timeline`))))

(fn `UserConstructionScript`
  (`self.K2_SetActorLocation` (`self.Actor`) (`SplineComponent.GetLocationAtSplinePoint` (`self.Spline`) 0 "World") false false))