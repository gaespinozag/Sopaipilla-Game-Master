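; BP_SopaipillaScore1 is a short-lived spinning sopaipilla actor that bursts into a reward effect.
; The construction script gives InterpToMovement a relative path from the origin to MovetoPso, while Tick applies constant yaw spin.
; BeginPlay waits briefly, spawns NS_Reward at the mesh, then destroys the actor.
; Overlap is empty; the scoring, sound and save logic is disconnected and never runs.
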(event `self.ReceiveBeginPlay`
  (`KismetSystemLibrary.Delay` 2.5)
  (`NiagaraFunctionLibrary.SpawnSystemAtLocation` "/Game/VFX/NiagaraSystem/Sopaipilla/NS_Reward.NS_Reward" (`SceneComponent.K2_GetComponentLocation` (`self.Mesh`)) (`SceneComponent.K2_GetComponentRotation` (`self.Mesh`)))
  (`self.K2_DestroyActor`))

(event `self.ReceiveActorBeginOverlap`
  (params (OtherActor :type "Actor Object Reference")))

(event `self.ReceiveTick`
  (params (DeltaSeconds :type "Float (single-precision)"))
  (`self.K2_AddActorLocalRotation` (`KismetMathLibrary.MakeRotator` 0.0 0.0 (* DeltaSeconds (`self.Rotation`)))))

(fn `UserConstructionScript`
  (`InterpToMovementComponent.AddControlPointPosition` (`self.InterpToMovement`) (0.0 0.0 0.0) true)
  (`InterpToMovementComponent.AddControlPointPosition` (`self.InterpToMovement`) (`self.MovetoPso`) true))