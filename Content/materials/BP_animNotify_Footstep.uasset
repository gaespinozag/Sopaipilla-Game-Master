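; Animation notify that plays a footstep sound cue chosen by the surface beneath the animated mesh's owner.
; On notify, it traces down from the owner's location along its negative up vector on the Visibility channel.
; The hit's surface type selects Platform or Wood audio, with Water reusing Wood and Gravel as the default.
; Sounds play at the world origin, not at the owner or impact point.
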(fn `Received_Notify`
  (params (MeshComp :type "SkeletalMeshComponent Object Reference") (Animation :type "AnimSequenceBase Object Reference") (EventReference :type "AnimNotifyEventReference Structure (by ref)"))
  (returns (ReturnValue :type Boolean))
  (bind _returnvalue (`ActorComponent.GetOwner` MeshComp))
  (bind _returnvalue_2 (`Actor.K2_GetActorLocation` _returnvalue))
  (bind _outhit (`KismetSystemLibrary.LineTraceSingle` _returnvalue_2 (+ _returnvalue_2 (* (`Actor.GetActorUpVector` _returnvalue) -200.0)) "TraceTypeQuery1"))
  (switch `EPhysicalSurface` (`GameplayStatics.GetSurfaceType` _outhit)
    (:`SurfaceType_Default`
      (`GameplayStatics.PlaySoundAtLocation` "/Game/Sounds/Footsteps/FootStep_Gravel_Stone/Sounds/Footstep_Gravel_SC.Footstep_Gravel_SC" (0.0 0.0 0.0) (struct) 1.0 1.0 0.0 null null null null))
    (:`SurfaceType1`
      (`GameplayStatics.PlaySoundAtLocation` "/Game/Sounds/Footsteps/FootStep_Platform/Sounds/Footstep_Platform_SC.Footstep_Platform_SC" (0.0 0.0 0.0) (struct) 1.0 1.0 0.0 null null null null))
    (:`SurfaceType2`
      (`GameplayStatics.PlaySoundAtLocation` "/Game/Sounds/Footsteps/FootStep_Wood/Sounds/Footstep_Wood_SC.Footstep_Wood_SC" (0.0 0.0 0.0) (struct) 1.0 1.0 0.0 null null null null))
    (:`SurfaceType3`
      (`GameplayStatics.PlaySoundAtLocation` "/Game/Sounds/Footsteps/FootStep_Wood/Sounds/Footstep_Wood_SC.Footstep_Wood_SC" (0.0 0.0 0.0) (struct) 1.0 1.0 0.0 null null null null)))
  (return false))